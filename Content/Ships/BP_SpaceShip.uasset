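; BP_SpaceShip is a player-controlled spaceship flown with Enhanced Input, using a mapping context it adds on BeginPlay.
; Force input pushes the static mesh along the ship's forward vector as an acceleration, scaled by VelocityFactor.
; Mouse input applies local pitch and yaw, and a separate input applies roll.
; Holding boost triples VelocityFactor and plays a timeline that changes camera FOV, which reverses on release.
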(event `self.ReceiveBeginPlay`
  (`EnhancedInputSubsystemInterface.AddMappingContext` (pcsubsystem `EnhancedInputLocalPlayerSubsystem` (`GameplayStatics.GetPlayerController` 0)) "/CosmicArchitect/InputMapping/IMC_SpaceShip.IMC_SpaceShip" 0 (struct)))

(event `EnhancedInput|/CosmicArchitect/Inputs/IA_Force`
  (params (ActionValue :type "Float (double-precision)") (ElapsedSeconds :type "Float (double-precision)") (TriggeredSeconds :type "Float (double-precision)") (InputAction :type "InputAction Object Reference" :default "/CosmicArchitect/Inputs/IA_Force.IA_Force"))
  (:`Triggered`
    (`PrimitiveComponent.AddForce` (`self.StaticMesh`) (* (* (`self.GetActorForwardVector`) (`self.VelocityFactor`)) ActionValue) "None" true)))

(event `EnhancedInput|/CosmicArchitect/Inputs/IA_Mouse`
  (params (ActionValue :type "Vector2D Structure") (ElapsedSeconds :type "Float (double-precision)") (TriggeredSeconds :type "Float (double-precision)") (InputAction :type "InputAction Object Reference" :default "/CosmicArchitect/Inputs/IA_Mouse.IA_Mouse"))
  (:`Triggered`
    (`self.K2_AddActorLocalRotation` (`KismetMathLibrary.MakeRotator` 0.0 (* ActionValue_Y 2.0) (* ActionValue_X 2.0)))))

(event `EnhancedInput|/CosmicArchitect/Inputs/IA_Roll`
  (params (ActionValue :type "Float (double-precision)") (ElapsedSeconds :type "Float (double-precision)") (TriggeredSeconds :type "Float (double-precision)") (InputAction :type "InputAction Object Reference" :default "/CosmicArchitect/Inputs/IA_Roll.IA_Roll"))
  (:`Triggered`
    (`self.K2_AddActorLocalRotation` (`KismetMathLibrary.MakeRotator` (* ActionValue 2.0)))))

(event `EnhancedInput|/CosmicArchitect/Inputs/IA_Boost`
  (params (ActionValue :type Boolean) (ElapsedSeconds :type "Float (double-precision)") (TriggeredSeconds :type "Float (double-precision)") (InputAction :type "InputAction Object Reference" :default "/CosmicArchitect/Inputs/IA_Boost.IA_Boost"))
  (:`Started`
    (set `self.VelocityFactor` 15000.0)
    (bind (_direction _zoomfov) (`Timeline|BoostEffect` :!label _label)
      (:`Update`
        (`CameraComponent.SetFieldOfView` (`self.Camera`) _zoomfov))))
  (:`Completed`
    (set `self.VelocityFactor` 5000.0)
    (goto _label :!via `Reverse`)))

(fn `UserConstructionScript`)